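; Tank enemy Blueprint that configures its movement speed from shared enemy data when play begins.
; It looks up its row in DT_Enemies_Values by its first actor tag, stores the values and applies the velocity as max walk speed.
; Pawn sensing is intentionally inert; disconnected legacy nodes that wrote target and player sightings to the AI Blackboard remain unused.
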(event `self.ReceiveBeginPlay`
  (bind (_enemyvalues_hp _enemyvalues_damage _enemyvalues_attackdelay _enemyvalues_attackspeed _enemyvalues_velocity) (break `/Game/Programming/Francesco/Enemies/Data/ST_Enemies_Stats` (`self.enemyValues`)))
  (bind _returnvalue (`|GetDataTableRow` "/Game/Programming/Francesco/Enemies/Data/DT_Enemies_Values.DT_Enemies_Values" (`|GetArrayItem` (`self.Tags`)))
    (:`then`
      (set `self.enemyValues` _returnvalue)
      (set `CharacterMovementComponent.MaxWalkSpeed` (`KismetMathLibrary.Conv_IntToDouble` _enemyvalues_velocity) (`self.CharacterMovement`)))))

(event `self.PawnSensing.OnSeePawn`
  (params (Pawn :type "Pawn Object Reference"))
  ;[0.02083 0.02083 0.02083] This enemy doesn't need to do anything OnSeePawn
)

(fn `UserConstructionScript`)