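; BP_Enemy_Fast is the fast enemy Blueprint, which loads its stats and flags when it sees the player.
; On BeginPlay, its first tag selects the row in DT_Enemies_Values stored as EnemyValues.
; PawnSensing sets the blackboard's player-seen flag, and a short retriggerable delay clears it once sightings stop.
; Disconnected legacy nodes for BP_Target sensing and positioning remain unused.
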(event `self.ReceiveBeginPlay`
  (bind _returnvalue (`|GetDataTableRow` "/Game/Programming/Francesco/Enemies/Data/DT_Enemies_Values.DT_Enemies_Values" (`|GetArrayItem` (`self.Tags`)))
    (:`then`
      (set `self.enemyValues` _returnvalue))))

(event `self.PawnSensing.OnSeePawn`
  (params (Pawn :type "Pawn Object Reference"))
  (bind (_returnvalue _returnvalue2) (`self.GetBooleanFromBlackboard`))
  (bind (_returnvalue_2 _returnvalue2_2) (`self.GetBooleanFromBlackboard`))
  (cast `/Game/ThirdPerson/Blueprints/BP_ThirdPersonCharacter` Pawn)
  (`BlackboardComponent.SetValueAsBool` _returnvalue _returnvalue2 true)
  (`KismetSystemLibrary.RetriggerableDelay` 0.6)
  (`BlackboardComponent.SetValueAsBool` _returnvalue_2 _returnvalue2_2 false))

(fn `UserConstructionScript`)