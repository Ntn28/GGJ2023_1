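; BP_Enemy is a melee enemy base that attacks with left or right hand sphere colliders, applying damage on overlap.
; Attack picks a random side, sphere-traces around itself, and plays an attack montage section on finding the third-person character or a BP_Target.
; A separate PlayMontage event uses a DoOnce gate to enable that side's collider, play the montage at configured speed, then disable both after a zero-length delay.
; Die is an empty stub.
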(event `PlayMontage`
  (bind (_enemyvalues_hp _enemyvalues_damage _enemyvalues_attackdelay _enemyvalues_attackspeed) (break `/Game/Programming/Francesco/Enemies/Data/ST_Enemies_Stats` (`self.enemyValues`)))
  (`/Engine/EditorBlueprintResources/StandardMacros.DoOnce` false :!label _label
    (:`Completed`
      (if (== (`self.attackSectionName`) "AttackR")
        (`PrimitiveComponent.SetCollisionEnabled` (`self.rSphereCollider`) "QueryAndPhysics")
        (else
          (`PrimitiveComponent.SetCollisionEnabled` (`self.lSphereCollider`) "QueryAndPhysics")))
      (`self.PlayAnimMontage` self "/Game/Programming/Francesco/Animations/IA_Animation/Attack/Base/BaseAttackMontage.BaseAttackMontage" _enemyvalues_attackspeed (`KismetSystemLibrary.MakeLiteralName` (`self.attackSectionName`)))
      (`KismetSystemLibrary.Delay` 0.0)
      (`PrimitiveComponent.SetCollisionEnabled` (`self.lSphereCollider`) "NoCollision")
      (`PrimitiveComponent.SetCollisionEnabled` (`self.rSphereCollider`) "NoCollision")
      (goto _label :!via `Reset`))))

(event `self.ReceiveBeginPlay`
  (`PrimitiveComponent.SetCollisionEnabled` (`self.lSphereCollider`) "NoCollision")
  (`PrimitiveComponent.SetCollisionEnabled` (`self.rSphereCollider`) "NoCollision"))

(event `self.rSphereCollider.OnComponentBeginOverlap`
  (params (OverlappedComponent :type "PrimitiveComponent Object Reference") (OtherActor :type "Actor Object Reference") (OtherComp :type "PrimitiveComponent Object Reference") (OtherBodyIndex :type Integer) (bFromSweep :type Boolean) (SweepResult :type "HitResult Structure (by ref)"))
  (bind (_enemyvalues_hp _enemyvalues_damage) (break `/Game/Programming/Francesco/Enemies/Data/ST_Enemies_Stats` (`self.enemyValues`)))
  (`GameplayStatics.ApplyDamage` OtherActor (`KismetMathLibrary.Conv_ByteToDouble` _enemyvalues_damage)))

(event `self.lSphereCollider.OnComponentBeginOverlap`
  (params (OverlappedComponent :type "PrimitiveComponent Object Reference") (OtherActor :type "Actor Object Reference") (OtherComp :type "PrimitiveComponent Object Reference") (OtherBodyIndex :type Integer) (bFromSweep :type Boolean) (SweepResult :type "HitResult Structure (by ref)"))
  (bind (_enemyvalues_hp _enemyvalues_damage) (break `/Game/Programming/Francesco/Enemies/Data/ST_Enemies_Stats` (`self.enemyValues`)))
  (`GameplayStatics.ApplyDamage` OtherActor (`KismetMathLibrary.Conv_ByteToDouble` _enemyvalues_damage)))

(fn `Attack`
  (bind _returnvalue (`self.K2_GetActorLocation`))
  (if (`KismetMathLibrary.RandomBool`)
    (set `self.attackSectionName` "AttackL")
    (else
      (set `self.attackSectionName` "AttackR")))
  (bind (_outhits _returnvalue_2) (`KismetSystemLibrary.SphereTraceMultiForObjects` :`Start` _returnvalue :`End` _returnvalue :`Radius` 120.0 :`ObjectTypes` (`|MakeArray` "ObjectTypeQuery3" "ObjectTypeQuery1" :!type "EObjectTypeQuery Enum") :`DrawDebugType` "ForDuration"))
  (if _returnvalue_2
    (for _index (range (+ (`KismetArrayLibrary.Array_Length` _outhits) 1))
      (bind (_output_bblockinghit _output_binitialoverlap _output_time _output_distance _output_location _output_impactpoint _output_normal _output_impactnormal _output_physmat _output_hitactor) (`GameplayStatics.BreakHitResult` (`|GetArrayItem` _outhits _index)))
      (cast `/Game/ThirdPerson/Blueprints/BP_ThirdPersonCharacter` _output_hitactor
        (:`then`
          _)
        (:`CastFailed`
          (cast `/Game/Programming/Francesco/Prorotypes/BP_Target` _output_hitactor)))
      (`self.PlayAnimMontage` "/Game/Programming/Alessandro/Animation_ForFrancesco/AI_Animation/Attack/IA_BaseAttack.IA_BaseAttack" 1.0 (`self.attackSectionName`))
      (break))))

(fn `Die`)

(fn `UserConstructionScript`)