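; Base AI Blueprint, by its name, that drives a chase-then-attack behavior against the player through blackboard keys.
; When PawnSensing sees any pawn outside Attack, it sets Chase, targets player character 0 and starts a looping timer.
; The timer polls horizontal distance to the player, switching Chase to Attack at close range and clearing itself.
; Nothing here resets Attack or performs movement.
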(event `self.PawnSensing.OnSeePawn`
  (params (Pawn :type "Pawn Object Reference"))
  (if (not (`BlackboardComponent.GetValueAsBool` (`AIBlueprintHelperLibrary.GetBlackboard` (`AIBlueprintHelperLibrary.GetAIController` self)) "Attack"))
    (`BlackboardComponent.SetValueAsBool` (`AIBlueprintHelperLibrary.GetBlackboard` (`AIBlueprintHelperLibrary.GetAIController` self)) "Chase" true)
    (`BlackboardComponent.SetValueAsObject` (`AIBlueprintHelperLibrary.GetBlackboard` (`AIBlueprintHelperLibrary.GetAIController` self)) "Target" (`GameplayStatics.GetPlayerCharacter` 0))
    (bind _returnvalue (`KismetSystemLibrary.K2_SetTimerDelegate` (delegate `HasToAttack?`) 0.1 true))
    (set `self.Timer` _returnvalue)))

(event `HasToAttack?`
  (if (< (`KismetMathLibrary.Abs` (`KismetMathLibrary.VSizeXY` (- (`self.K2_GetActorLocation` (`GameplayStatics.GetPlayerCharacter` 0)) (`self.K2_GetActorLocation`)))) 120.0)
    (`BlackboardComponent.SetValueAsBool` (`AIBlueprintHelperLibrary.GetBlackboard` (`AIBlueprintHelperLibrary.GetAIController` self)) "Chase" false)
    (`BlackboardComponent.SetValueAsBool` (`AIBlueprintHelperLibrary.GetBlackboard` (`AIBlueprintHelperLibrary.GetAIController` self)) "Attack" true)
    (`KismetSystemLibrary.K2_ClearAndInvalidateTimerHandle` (`self.Timer`))))

(fn `UserConstructionScript`)